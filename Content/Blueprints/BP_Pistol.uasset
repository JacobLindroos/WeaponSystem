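; BP_Pistol is a pistol actor that shows a floating name label when the player is nearby.
; Each Tick measures the distance to player character 0 and shows the TextRender between 50 and 300 units, turning it toward the player.
; Outside that band the label is hidden, with very close range treated as the weapon being equipped.
; The Blueprint contains no firing or pickup logic.
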(event `self.ReceiveTick`
  (params (DeltaSeconds :type "Float (single-precision)"))
  (bind _textrender (`self.TextRender`))
  (bind _returnvalue (`KismetMathLibrary.VSize` (- (`self.K2_GetActorLocation` (`GameplayStatics.GetPlayerCharacter` 0)) (`self.K2_GetActorLocation`))))
  ;[1 0.8296 0.403] Displays gun name if player is within 300 units from gun, else if 50 within the name is not displayed cause wepaon is eqipped
  (if (< _returnvalue 300.0)
    (if (< _returnvalue 50.0)
      (`SceneComponent.SetVisibility` _textrender false false :!label _label)
      (else
        (`SceneComponent.SetVisibility` _textrender true false)
        (`SceneComponent.K2_SetWorldRotation` (`self.TextRender`) (`KismetMathLibrary.FindLookAtRotation` (`self.K2_GetActorLocation`) (`self.K2_GetActorLocation` (`GameplayStatics.GetPlayerCharacter` 0))) false false)))
    (else
      (goto _label))))

(fn `UserConstructionScript`
  (`parent.UserConstructionScript`))